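; Proximity-triggered video actor that lets the player show and play the MS_WH media source on a plane.
; BeginPlay opens the source, and any overlap with the box enables player input and shows a text render.
; The F key uses a FlipFlop to alternate between showing and playing the video and hiding and pausing it.
; Ending overlap disables input, hides plane and text, and pauses playback without resetting the FlipFlop.
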(event OnComponentBeginOverlap(Box)
  (params (OverlappedComponent :type Primitive%20Component%20Object%20Reference) (OtherActor :type Actor%20Object%20Reference) (OtherComp :type Primitive%20Component%20Object%20Reference) (OtherBodyIndex :type Integer) (bFromSweep :type Boolean) (SweepResult :type Hit%20Result%20Structure%20%28by%20ref%29))
  (Input|EnableInput (Game|GetPlayerController 0))
  (Rendering|SetVisibility (Variables|Default|GetTextRender) true false))

(event OnComponentEndOverlap(Box)
  (params (OverlappedComponent :type Primitive%20Component%20Object%20Reference) (OtherActor :type Actor%20Object%20Reference) (OtherComp :type Primitive%20Component%20Object%20Reference) (OtherBodyIndex :type Integer))
  (Input|DisableInput (Game|GetPlayerController 0))
  (Rendering|SetVisibility (Variables|Default|GetPlane) false false)
  (Sequencer|Player|Pause (Variables|Default|GetMediaPlayer))
  (Rendering|SetVisibility (Variables|Default|GetTextRender) false false))

(event EventBeginPlay
  (Media|MediaPlayer|OpenSource (Variables|Default|GetMediaPlayer) "/Game/Movies/MS_WH.MS_WH"))

(event Input|KeyboardEvents|F
  (params (Key :type Key%20Structure :default "None"))
  (bind _plane (Variables|Default|GetPlane))
  (bind _mediaplayer (Variables|Default|GetMediaPlayer))
  (:Pressed
    (Utilities|FlowControl|FlipFlop
      (:A
        (Rendering|SetVisibility _plane true false)
        (Media|MediaPlayer|Play _mediaplayer :!class /Script/MediaAssets.MediaPlayer))
      (:B
        (Rendering|SetVisibility _plane false false)
        (Sequencer|Player|Pause _mediaplayer)))))

(fn ConstructionScript)