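; BP_CameraScene is an item inspection stage that shows a given mesh alongside a UI_Introduce widget with its name and description.
; The inspect event takes input from the player, and holding either mouse button while moving rotates the mesh.
; The mouse wheel slides a SceneCaptureComponent2D along X as zoom.
; Closing the widget restores player input, destroys the first BP_CameraScene found and hides the cursor.
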(event Custom|Event_GuanBi
  (bind _returnvalue (Game|GetPlayerController 0))
  (Widget|RemovefromParent (Variables|Default|GetUI_Inspect))
  (Input|EnableInput (Variables|Default|GetPlayer) _returnvalue)
  (Input|DisableInput _returnvalue)
  (bind _returnvalue_2 (Actor|GetActorOfClass "BP_CameraScene_C"))
  (Utilities|IsValid _returnvalue_2
    (:Is%20Valid
      (Actor|DestroyActor _returnvalue_2)
      (Variables|/Script/Engine.PlayerController|SetbShowMouseCursor _returnvalue false))))

(event EventBeginPlay
  (Variables|/Script/Engine.PlayerController|SetbShowMouseCursor (Game|GetPlayerController 0) true))

(event Collision|EventActorBeginOverlap
  (params (OtherActor :type Actor%20Object%20Reference)))

(event EventTick
  (params (DeltaSeconds :type Float%20%28single-precision%29)))

(event EventInsper查看
  (params (Player :type BP%20Third%20Person%20Character%20Object%20Reference) (Name :type String) (Description :type String) (Mesh :type Static%20Mesh%20Object%20Reference))
  (bind _returnvalue (Game|GetPlayerController 0))
  (Variables|Default|SetPlayer Player)
  (Components|StaticMesh|SetStaticMesh (Variables|Default|GetStaticMesh) Mesh)
  (bind _returnvalue_2 (UserInterface|CreateWidget "/Game/Resources/BP/MeshCheck/UI/UI_Introduce.UI_Introduce_C" 0 Name Description))
  (bind _output_get (Variables|Default|SetUI_Inspect _returnvalue_2))
  (UserInterface|Viewport|AddtoViewport _output_get 0)
  (EventDispatchers|BindEventtoOnClicked (Variables|/Game/Resources/BP/MeshCheck/UI/UI_Introduce.UI_Introduce_C|GetButton_关闭 (Variables|Default|GetUI_Inspect)) (delegate Custom|Event_GuanBi))
  (Input|EnableInput _returnvalue)
  (Input|DisableInput (Variables|Default|GetPlayer) _returnvalue))

(event Input|MouseEvents|MouseX
  (params (AxisValue :type Float%20%28single-precision%29))
  (if (Variables|Default|GetisRotate？)
    (Transformation|SetWorldRotation (Variables|Default|GetStaticMesh) (Math|Rotator|CombineRotators (Transformation|GetWorldRotation (Variables|Default|GetStaticMesh)) (Math|Rotator|MakeRotator 0.0 0.0 (* AxisValue -5.0))) false false)))

(event Input|MouseEvents|MouseY
  (params (AxisValue :type Float%20%28single-precision%29))
  (if (Variables|Default|GetisRotate？)
    (Transformation|SetWorldRotation (Variables|Default|GetStaticMesh) (Math|Rotator|CombineRotators (Transformation|GetWorldRotation (Variables|Default|GetStaticMesh)) (Math|Rotator|MakeRotator 0.0 (* AxisValue -5.0) 0.0)) false false)))

(event Input|MouseEvents|MouseWheelAxis
  (params (AxisValue :type Float%20%28single-precision%29))
  (bind _returnvalue (* AxisValue 1e+01))
  (bind _scenecapturecomponent2d (Variables|Default|GetSceneCaptureComponent2D))
  (bind _scenecapturecomponent2d_2 (Variables|Default|GetSceneCaptureComponent2D))
  (if (!= AxisValue 0.0)
    (if (== AxisValue 1.0)
      (Transformation|SetRelativeLocation _scenecapturecomponent2d_2 (Math|Vector|MakeVector (+ _returnvalue (.x (Variables|/Script/Engine.SceneComponent|GetRelativeLocation _scenecapturecomponent2d_2))) 0.0 0.0) false false)
      (else
        (Transformation|SetRelativeLocation _scenecapturecomponent2d (Math|Vector|MakeVector (+ (.x (Variables|/Script/Engine.SceneComponent|GetRelativeLocation _scenecapturecomponent2d)) _returnvalue) 0.0 0.0) false false)))))

(event Input|MouseEvents|LeftMouseButton
  (params (Key :type Key%20Structure :default "None"))
  (:Pressed
    (Variables|Default|SetisRotate？ true))
  (:Released
    (Variables|Default|SetisRotate？ false)))

(event Input|MouseEvents|RightMouseButton
  (params (Key :type Key%20Structure :default "None"))
  (:Pressed
    (Variables|Default|SetisRotate？ true))
  (:Released
    (Variables|Default|SetisRotate？ false)))

(fn ConstructionScript)