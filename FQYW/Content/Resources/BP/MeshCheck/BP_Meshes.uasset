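; BP_Meshes is an interactable prop actor whose mesh can be inspected through a separate BP_CameraScene.
; Its construction script applies the configurable Mesh, and a sphere overlap with BP_ThirdPersonCharacter toggles input and the prompt widget.
; On Interact, it destroys any existing BP_CameraScene, spawns a new one far off in the world and passes it the player, name, description and mesh.
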(event OnComponentBeginOverlap(Sphere)
  (params (OverlappedComponent :type Primitive%20Component%20Object%20Reference) (OtherActor :type Actor%20Object%20Reference) (OtherComp :type Primitive%20Component%20Object%20Reference) (OtherBodyIndex :type Integer) (bFromSweep :type Boolean) (SweepResult :type Hit%20Result%20Structure%20%28by%20ref%29))
  (Utilities|Casting|CastToBP_ThirdPersonCharacter OtherActor)
  (Input|EnableInput (Game|GetPlayerController 0))
  (Rendering|SetVisibility (Variables|Default|GetWidget) true false))

(event OnComponentEndOverlap(Sphere)
  (params (OverlappedComponent :type Primitive%20Component%20Object%20Reference) (OtherActor :type Actor%20Object%20Reference) (OtherComp :type Primitive%20Component%20Object%20Reference) (OtherBodyIndex :type Integer))
  (Utilities|Casting|CastToBP_ThirdPersonCharacter OtherActor)
  (Input|DisableInput (Game|GetPlayerController 0))
  (Rendering|SetVisibility (Variables|Default|GetWidget) false false))

(event EventBeginPlay)

(event Collision|EventActorBeginOverlap
  (params (OtherActor :type Actor%20Object%20Reference)))

(event EventTick
  (params (DeltaSeconds :type Float%20%28single-precision%29)))

(event EventInteract交互
  (params (Player :type BP%20Third%20Person%20Character%20Object%20Reference))
  (bind _returnvalue (Game|GetPlayerController 0))
  (bind _returnvalue_2 (Actor|GetActorOfClass "/Game/Resources/BP/MeshCheck/BP_CameraScene.BP_CameraScene_C"))
  (Utilities|IsValid _returnvalue_2
    (:Is%20Valid
      (Actor|DestroyActor _returnvalue_2))
    (:Is%20Not%20Valid
      _))
  (bind _returnvalue_3 (Game|SpawnActorfromClass "/Game/Resources/BP/MeshCheck/BP_CameraScene.BP_CameraScene_C" (Math|Transform|MakeTransform "50000000.000000, 0, 0") "Undefined" "OverrideRootScale" 0 0))
  (Class|BPIInspect|Insper查看(Message) _returnvalue_3 Player (Variables|Default|GetName) (Variables|Default|GetDescription) (Variables|/Script/Engine.StaticMeshComponent|GetStaticMesh (Variables|Default|GetStaticMesh)))
  (Input|EnableInput _returnvalue)
  (Input|DisableInput _returnvalue))

(fn ConstructionScript
  (Components|StaticMesh|SetStaticMesh (Variables|Default|GetStaticMesh) (Variables|Default|GetMesh)))