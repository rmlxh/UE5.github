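; BP_YWQ is a trigger-box actor that reveals a large group of skeletal mesh figures with sound.
; When anything begins overlapping the box, it plays the WuDao cue in 2D and makes dozens of skeletal mesh components visible at once.
; After a 17-second delay it plays a second 2D sound.
; The overlap has no actor filter or one-shot guard, and nothing hides the meshes again.
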(event OnComponentBeginOverlap(Box)
  (params (OverlappedComponent :type Primitive%20Component%20Object%20Reference) (OtherActor :type Actor%20Object%20Reference) (OtherComp :type Primitive%20Component%20Object%20Reference) (OtherBodyIndex :type Integer) (bFromSweep :type Boolean) (SweepResult :type Hit%20Result%20Structure%20%28by%20ref%29))
  (Audio|PlaySound2D "/Game/Resources/Sound/WuDao_Cue.WuDao_Cue" 1.0 1.0 0.0 0 0)
  (Rendering|SetVisibility (Variables|Default|GetSkeletalMesh64) true false)
  (Rendering|SetVisibility (Variables|Default|GetSkeletalMesh17) true false)
  (Rendering|SetVisibility (Variables|Default|GetSkeletalMesh50) true false)
  (Rendering|SetVisibility (Variables|Default|GetSkeletalMesh10) true false)
  (Utilities|FlowControl|Delay 17.0)
  (Audio|PlaySound2D (Variables|Default|Getsound) 1.0 1.0 0.0 0 0))

(fn ConstructionScript)